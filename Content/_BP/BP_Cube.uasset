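; BP_Cube is a physics cube that recursively splits into eight smaller copies of itself.
; After a random delay, it disables its physics and collision, spawns children at eight scene-component transforms with inherited scale, then destroys itself.
; Generation passes to children, offsetting material hue and limiting splits against a maximum each cube randomizes.
; Non-first cubes launch with a random impulse and briefly flash emissive through a dynamic material instance.
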(event Custom|StartSplit
  (bind _result (Math|Integer|IncrementInt (Variables|Default|GetGeneration))
    (:%20%20
      (if (<= _result (Variables|Default|GetMaxGenerations))
        (Utilities|FlowControl|Delay (Math|Random|RandomFloatinRange 1.0 4.0))
        (CallFunction|DissableParentCube)
        (CallFunction|SpawnCubes)))))

(event Custom|SpawnCubes
  (for _array_element (Variables|Default|GetSpawnLocation)
    (Game|SpawnActorfromClass "BP_Cube_C" (Math|Transform|MakeTransform (Transformation|GetWorldLocation _array_element) (Transformation|GetWorldRotation _array_element) (* (Variables|/Script/Engine.SceneComponent|GetRelativeScale3D _array_element) (Transformation|GetActorScale3D))) "AlwaysSpawn" "MultiplyWithRoot" 0 (Variables|Default|GetGeneration) 0))
  (Actor|DestroyActor))

(event EventBeginPlay
  (Utilities|FlowControl|Delay 1.0)
  (|AddSceneComponents)
  (bind _returnvalue (Rendering|Material|CreateDynamicMaterialInstance (Variables|Default|GetCube) 0 "/Game/_MAT/MI_Cube.MI_Cube" "None" :!class /Script/Engine.PrimitiveComponent))
  (bind _output_get (Variables|Default|SetMID_Cube _returnvalue))
  (Rendering|Material|SetScalarParameterValue _output_get "HueOffset" (Math|Conversions|ToFloat(Integer) (Variables|Default|GetGeneration)) :!class /Script/Engine.MaterialInstanceDynamic)
  (Variables|Default|SetMaxGenerations (Math|Random|RandomIntegerinRange 1 4))
  (if (Variables|Default|GetFirstCube?)
    (CallFunction|StartSplit)
    (else
      (Physics|AddImpulse (Variables|Default|GetCube) (* (Math|Random|RandomUnitVector) (Variables|Default|GetInpulseScalar)) "None" true)
      (CallFunction|StartSplit)
      (Rendering|Material|SetScalarParameterValue (Variables|Default|GetMID_Cube) "Emission" 5.0 :!class /Script/Engine.MaterialInstanceDynamic)
      (Utilities|FlowControl|Delay 0.1)
      (Rendering|Material|SetScalarParameterValue (Variables|Default|GetMID_Cube) "Emission" 0.0 :!class /Script/Engine.MaterialInstanceDynamic))))

(fn ConstructionScript)

(fn DissableParentCube
  (bind _cube (Variables|Default|GetCube))
  (Physics|SetSimulatePhysics _cube false)
  (Collision|SetCollisionEnabled _cube "NoCollision")
  (Collision|SetCollisionObjectType _cube "ECC_WorldStatic"))